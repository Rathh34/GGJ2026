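; BP_Rope is an interactable pull rope that sets clouds in the level moving.
; Interaction calls MovingClouds, which uses a DoOnce so the pull happens a single time.
; The MovingSphere timeline, with its duration set by PlayRateS, lowers the Sphere handle while shifting the Cable.
; When it finishes, it calls Moving on every actor in the Cloud, CloudMove and CloudMask arrays.
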(event Custom|MovingClouds
  (Utilities|FlowControl|DoOnce false
    (:Completed
      (Components|Timeline|SetPlayRate (Variables|Default|GetMovingSphere) (/ 1.0 (Variables|Default|GetPlayRate%28s%29)))
      (bind _alpha (Timeline|MovingSphere PlayFromStart)
        (:Update
          (Transformation|SetRelativeLocation (Variables|Default|GetSphere) (Math|Vector|Lerp(Vector) "0, 0, 0" "0.000000,0.000000,-50.000000" _alpha) false false)
          (Transformation|SetRelativeLocation (Variables|Default|GetCable) (Math|Vector|Lerp(Vector) "0.000000,0.000000,200.000000" "0.000000,0.000000,225.000000" _alpha) false false))
        (:Finished
          (Utilities|FlowControl|Sequence
            (:then_0
              (for _array_element (Variables|Default|GetCloud)
                (Default|Moving _array_element)))
            (:then_1
              (for _array_element_2 (Variables|Default|GetCloudMove)
                (Default|Moving _array_element_2)))
            (:then_2
              (for _array_element_3 (Variables|Default|GetCloudMask)
                (Default|Moving _array_element_3)))))))))

(event EventInteraction
  (params (Interactor :type Actor%20Object%20Reference))
  (CallFunction|MovingClouds))

(fn ConstructionScript)