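; BP_DestructibleTest is a breakable actor, apparently a test, that shatters away from the player.
; Its Destruce event runs once, playing a camera shake and hit sound, disabling the box collision and enabling physics on the Geometry Collection.
; The impulse uses the unnormalized player-to-actor vector times ImpulseForce, so it scales with distance.
; It then triggers CameraShakeDestroy on the side-scrolling camera manager.
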(event EventDestruce
  (Utilities|FlowControl|DoOnce false
    (:Completed
      (Camera|PlayWorldCameraShake "/Game/BP_HitShake.BP_HitShake_C" "0, 0, 0" 0.0 5e+01 0.0)
      (Audio|PlaySound2D (Variables|Default|GetHit%20Sound) 1.0 1.0 0.0 0 0)
      (Collision|SetCollisionEnabled (Variables|Default|GetBox) "NoCollision")
      (Physics|SetSimulatePhysics (Variables|Default|GetGeometryCollection) true)
      (Physics|AddImpulse (Variables|Default|GetGeometryCollection) (* (- (Transformation|GetActorLocation) (Transformation|GetActorLocation (Game|Player|GetPlayerPawn 0))) (Variables|Default|GetImpulse%20Force)) "None" false)
      (bind _asbp_side_scrolling_camera_manager (Utilities|Casting|CastToBP_SideScrollingCameraManager (Game|GetPlayerCameraManager 0)))
      (Default|CameraShakeDestroy _asbp_side_scrolling_camera_manager))))

(fn ConstructionScript)