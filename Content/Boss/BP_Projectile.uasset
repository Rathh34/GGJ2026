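; Boss-fight projectile that flies at a configurable speed and destroys itself after a short lifetime or on its first collision.
; Hitting a living BP_SideScrollingCharacter resets the fight by replacing BP_MiniBoss with a fresh copy at the same transform, keeping its Camera reference.
; If a boss exists, that hit also sends HitMessage to the character and removes health bar widgets.
; Any impact spawns a small molotov particle effect.
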(event OnComponentHit(Sphere)
  (params (HitComponent :type Primitive%20Component%20Object%20Reference) (OtherActor :type Actor%20Object%20Reference) (OtherComp :type Primitive%20Component%20Object%20Reference) (NormalImpulse :type Vector :default "0, 0, 0") (Hit :type Hit%20Result%20Structure%20%28by%20ref%29))
  (Utilities|FlowControl|DoOnce false
    (:Completed
      (bind _asbp_side_scrolling_character (Utilities|Casting|CastToBP_SideScrollingCharacter OtherActor)
        (:then
          (if (Variables|/Game/Variant_SideScroller/Blueprints/BP_SideScrollingCharacter.BP_SideScrollingCharacter_C|GetDead? _asbp_side_scrolling_character)
            _
            (else
              (bind _returnvalue (Actor|GetActorOfClass "/Game/Boss/BP_MiniBoss.BP_MiniBoss_C"))
              (Utilities|IsValid _returnvalue
                (:Is%20Valid
                  (bind _returnvalue_2 (Game|SpawnActorfromClass "/Game/Boss/BP_MiniBoss.BP_MiniBoss_C" (Transformation|GetActorTransform _returnvalue) "Undefined" "MultiplyWithRoot" 0 0))
                  (Variables|/Game/Boss/BP_MiniBoss.BP_MiniBoss_C|SetCamera _returnvalue_2 (Variables|/Game/Boss/BP_MiniBoss.BP_MiniBoss_C|GetCamera _returnvalue))
                  (Actor|DestroyActor _returnvalue)
                  (Class|BPIHumanoid|Hit(Message) _asbp_side_scrolling_character 1.0)
                  (bind _foundwidgets (Widget|GetAllWidgetsOfClass "/Game/Boss/WBP_HealthBar.WBP_HealthBar_C" true))
                  (for _array_element _foundwidgets
                    (Widget|RemovefromParent _array_element)))
                (:Is%20Not%20Valid
                  _)))))
        (:CastFailed
          _))
      (Effects|SpawnEmitteratLocation "/Game/Realistic_Starter_VFX_Pack_Vol2/Particles/Explosion/P_MolotovNoDetail.P_MolotovNoDetail" (Transformation|GetActorLocation) "0, 0, 0" "0.500000,0.500000,0.500000")
      (Actor|DestroyActor))))

(event EventBeginPlay
  (bind _projectilemovement (Variables|Default|GetProjectileMovement))
  (bind _speed (Variables|Default|GetSpeed))
  (Variables|/Script/Engine.ProjectileMovementComponent|SetInitialSpeed _projectilemovement _speed)
  (Variables|/Script/Engine.ProjectileMovementComponent|SetMaxSpeed _projectilemovement _speed)
  (Utilities|FlowControl|Delay 5.0)
  (Actor|DestroyActor))

(fn ConstructionScript)